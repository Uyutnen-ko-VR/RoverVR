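; Radar actor that the rover repairs through a timing minigame.
; Rover overlap reveals MinigameSphere, which Tick bounces vertically with MoveComponentTo.
; Either trigger input calls OnRadarFixedEvent while InPlace is set by the sphere entering MinigameTrigger; OnRadarFixed_Event moves AntennaHandler and starts the dish mesh spinning.
; End overlap compares OverlappedComponent rather than OtherComp to the sphere, so InPlace stays set after the first entry.
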(event `OnRadarFixed_Event`
  (bind _antennahandler (`self.AntennaHandler`))
  (bind _returnvalue_location (`KismetMathLibrary.BreakTransform` (`SceneComponent.GetRelativeTransform` _antennahandler)))
  (`KismetSystemLibrary.MoveComponentTo` _antennahandler _returnvalue_location (struct) false false 0.5)
  (set `self.bFixed` true))

(event `self.ReceiveTick`
  (params (DeltaSeconds :type "Float (single-precision)"))
  (bind _minigamesphere (`self.MinigameSphere`))
  (bind _returnvalue (`SceneComponent.GetRelativeTransform` _minigamesphere))
  (`|ExecutionSequence`
    (:`then_0`
      (if (`self.bFixed`)
        (`SceneComponent.K2_AddRelativeRotation` (`self.5g__1__Sphere_001`) (struct :`Yaw` 1.0) false false)))
    (:`then_1`
      (if (`self.bFixing`)
        (if (== (.z (.location _returnvalue)) 100.0)
          (`KismetSystemLibrary.MoveComponentTo` _minigamesphere (`KismetMathLibrary.MakeVector` (.x (.location _returnvalue)) (.y (.location _returnvalue)) 3000.0) (.rotation _returnvalue) false false 3.0 :!label _label)
          (elif (== (.z (.location _returnvalue)) 3000.0)
            (`KismetSystemLibrary.MoveComponentTo` _minigamesphere (`KismetMathLibrary.MakeVector` (.x (.location _returnvalue)) (.y (.location _returnvalue)) 100.0) (.rotation _returnvalue) false false 3.0)))))))

(event `self.RoverTrigger.OnComponentBeginOverlap`
  (params (OverlappedComponent :type "PrimitiveComponent Object Reference") (OtherActor :type "Actor Object Reference") (OtherComp :type "PrimitiveComponent Object Reference") (OtherBodyIndex :type Integer) (bFromSweep :type Boolean) (SweepResult :type "HitResult Structure (by ref)"))
  (cast `/Game/Blueprints/Rover/BP_Rover` OtherActor)
  (set `self.bFixing` true)
  (`SceneComponent.SetHiddenInGame` (`self.MinigameSphere`) false false)
  (goto _label))

(event `InputAction|TriggerRight`
  (params (Key :type "Key Structure"))
  (:`Pressed`
    (`KismetSystemLibrary.PrintString` "Hello")
    (if (`self.bInPlace`) :!label _label_2
      (`self.OnRadarFixed_Event`))))

(event `InputAction|TriggerLeft`
  (params (Key :type "Key Structure"))
  (:`Pressed`
    (`KismetSystemLibrary.PrintString` "Hello")
    (goto _label_2)))

(event `self.MinigameTrigger.OnComponentBeginOverlap`
  (params (OverlappedComponent :type "PrimitiveComponent Object Reference") (OtherActor :type "Actor Object Reference") (OtherComp :type "PrimitiveComponent Object Reference") (OtherBodyIndex :type Integer) (bFromSweep :type Boolean) (SweepResult :type "HitResult Structure (by ref)"))
  (if (== OtherComp (`self.MinigameSphere`))
    (set `self.bInPlace` true)))

(event `self.MinigameTrigger.OnComponentEndOverlap`
  (params (OverlappedComponent :type "PrimitiveComponent Object Reference") (OtherActor :type "Actor Object Reference") (OtherComp :type "PrimitiveComponent Object Reference") (OtherBodyIndex :type Integer))
  (if (== OverlappedComponent (`self.MinigameSphere`))
    (set `self.bInPlace` false)))

(fn `UserConstructionScript`)