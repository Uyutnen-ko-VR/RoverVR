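; Explorer is a test actor that drives its physics Cube at a constant speed along world X and reports that speed.
; Each Tick it overwrites the Cube's linear velocity, then reads it back.
; When the velocity is nonzero, it converts the magnitude from cm/s to km/h and prints it as a debug string.
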(event `self.ReceiveBeginPlay`)

(event `self.ReceiveTick`
  (params (DeltaSeconds :type "Float (single-precision)"))
  (`|ExecutionSequence`
    (:`then_0`
      (`PrimitiveComponent.SetPhysicsLinearVelocity` (`self.Cube`) (1000.0 0.0 0.0) false "None"))
    (:`then_1`
      (bind _returnvalue (`PrimitiveComponent.GetPhysicsLinearVelocity` (`self.Cube`) "None"))
      (if (!= _returnvalue (0.0 0.0 0.0))
        (`KismetSystemLibrary.PrintString` (`KismetStringLibrary.Conv_DoubleToString` (* (* (`KismetMathLibrary.VSize` _returnvalue) 0.01) 3.6)))))))

(fn `UserConstructionScript`)