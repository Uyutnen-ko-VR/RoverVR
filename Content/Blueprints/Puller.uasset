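; Puller is a grabbable VR lever or switch that exposes an On state, starting off.
; Grab stores the motion controller, and Tick pitches the Cube toward it using a look-at in the Cube's rotated local space, clamped to a symmetric range.
; Release clears the controller and snaps the Cube to either limit, setting On according to a pitch threshold.
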(event `self.ReceiveBeginPlay`
  (set `self.On` false))

(event `/Game/Interfaces/Grab.Release`
  (params (MotionController :type "MotionControllerComponent Object Reference"))
  (if (not (== null (`self.Motion Controller`)))
    (set `self.Motion Controller` null)
    (if (> (.pitch (.rotation (`SceneComponent.GetRelativeTransform` (`self.Cube`)))) 10.0)
      (set `self.On` true)
      (`SceneComponent.K2_SetRelativeRotation` (`self.Cube`) (struct :`Pitch` 40.0) false false)
      (else
        (set `self.On` false)
        (`SceneComponent.K2_SetRelativeRotation` (`self.Cube`) (struct :`Pitch` -40.0) false false)))))

(event `/Game/Interfaces/Grab.Grab`
  (params (MotionController :type "MotionControllerComponent Object Reference"))
  (set `self.Motion Controller` MotionController))

(event `self.ReceiveTick`
  (params (DeltaSeconds :type "Float (single-precision)"))
  (bind _cube (`self.Cube`))
  (bind (_returnvalue_location _returnvalue_rotation _returnvalue_scale) (`KismetMathLibrary.BreakTransform` (`SceneComponent.K2_GetComponentToWorld` (`self.Cube`))))
  (bind _motion_controller (`self.Motion Controller`)
    (:`then`
      (bind _returnvalue_location_2 (`KismetMathLibrary.BreakTransform` (`KismetMathLibrary.MakeRelativeTransform` (`SceneComponent.K2_GetComponentToWorld` _motion_controller) (`KismetMathLibrary.MakeTransform` _returnvalue_location (`KismetMathLibrary.ComposeRotators` _returnvalue_rotation (struct :`Pitch` 90.0)) _returnvalue_scale))))
      (bind (_returnvalue_roll _returnvalue_pitch) (`KismetMathLibrary.BreakRotator` (`KismetMathLibrary.FindLookAtRotation` (`KismetMathLibrary.MakeVector` 0.0) _returnvalue_location_2)))
      (`SceneComponent.K2_SetRelativeRotation` _cube (`KismetMathLibrary.MakeRotator` 0.0 (`KismetMathLibrary.FClamp` (+ (.pitch (.rotation (`SceneComponent.GetRelativeTransform` _cube))) _returnvalue_pitch) -40.0 40.0)) false false))
    (:`else`)))

(fn `UserConstructionScript`)