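; Lever1 is a motion-controller-grabbable lever that feeds X and Y rotation input to the BP_mooner actor found at BeginPlay.
; While grabbed, Tick rotates the Cube pivot toward the controller with clamped roll and pitch.
; When Con is on, the Handle's world-space X/Y offset from the pivot is scaled and written to the mooner's XRot and YRot.
; Release can clear the controller, reset the pivot and zero both values.
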(event `self.ReceiveBeginPlay`
  (bind _returnvalue (`GameplayStatics.GetActorOfClass` "/Game/Blueprints/BP_mooner.BP_mooner_C"))
  (set `self.Explorer` _returnvalue))

(event `/Game/Interfaces/Grab.Release`
  (params (MotionController :type "MotionControllerComponent Object Reference"))
  (bind _explorer (`self.Explorer`))
  (if (not (== null (`self.Motion Controller`)))
    (set `self.Motion Controller` null)
    (`SceneComponent.K2_SetWorldRotation` (`self.Cube`) (struct :`Pitch` 90.0) false false)
    (set `self.XRot` 0.0)
    (set `self.YRot` 0.0)
    (set `/Game/Blueprints/BP_mooner.XRot` 0.0 _explorer)
    (set `/Game/Blueprints/BP_mooner.YRot` 0.0 _explorer)))

(event `/Game/Interfaces/Grab.Grab`
  (params (MotionController :type "MotionControllerComponent Object Reference"))
  (set `self.Motion Controller` MotionController))

(event `self.ReceiveTick`
  (params (DeltaSeconds :type "Float (single-precision)"))
  (bind _explorer (`self.Explorer`))
  (bind _cube (`self.Cube`))
  (`|ExecutionSequence`
    (:`then_0`
      (bind _motion_controller (`self.Motion Controller`)
        (:`then`
          (`SceneComponent.K2_SetWorldRotation` _cube (`KismetMathLibrary.MakeRotator` (`KismetMathLibrary.FClamp` (.roll (`KismetMathLibrary.FindLookAtRotation` (`SceneComponent.K2_GetComponentLocation` _cube) (`SceneComponent.K2_GetComponentLocation` _motion_controller))) 0.0 180.0) (`KismetMathLibrary.FClamp` (.pitch (`KismetMathLibrary.FindLookAtRotation` (`SceneComponent.K2_GetComponentLocation` _cube) (`SceneComponent.K2_GetComponentLocation` _motion_controller))) 0.0 150.0) (.yaw (`KismetMathLibrary.FindLookAtRotation` (`SceneComponent.K2_GetComponentLocation` _cube) (`SceneComponent.K2_GetComponentLocation` _motion_controller)))) false false))
        (:`else`)))
    (:`then_1`
      (if (`/Game/Blueprints/Puller.On` (`self.con`))
        (bind _output_get (set `self.XRot` (/ (.x (- (`SceneComponent.K2_GetComponentLocation` (`self.Handle`)) (`SceneComponent.K2_GetComponentLocation` (`self.Cube`)))) 20.0)))
        (bind _output_get_2 (set `self.YRot` (/ (.y (- (`SceneComponent.K2_GetComponentLocation` (`self.Handle`)) (`SceneComponent.K2_GetComponentLocation` (`self.Cube`)))) 20.0)))
        (set `/Game/Blueprints/BP_mooner.XRot` _output_get _explorer)
        (set `/Game/Blueprints/BP_mooner.YRot` _output_get_2 _explorer)))))

(fn `UserConstructionScript`)