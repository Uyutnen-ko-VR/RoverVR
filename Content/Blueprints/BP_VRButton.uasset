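; BP_VRButton is a physical VR button that sends its Color to the level's BP_Rover when pressed.
; A VRPawn overlapping its Box sinks the Button mesh, fires OnButtonPressedEvent on the rover found at BeginPlay, then raises the mesh.
; IsPressable blocks re-triggering during the animation but clears before the pawn cast, so any other overlapping actor leaves the button locked.
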(event `self.ReceiveBeginPlay`
  (bind _returnvalue (`GameplayStatics.GetActorOfClass` "/Game/Blueprints/Rover/BP_Rover.BP_Rover_C"))
  (set `self.Rover` _returnvalue))

(event `self.Box.OnComponentBeginOverlap`
  (params (OverlappedComponent :type "PrimitiveComponent Object Reference") (OtherActor :type "Actor Object Reference") (OtherComp :type "PrimitiveComponent Object Reference") (OtherBodyIndex :type Integer) (bFromSweep :type Boolean) (SweepResult :type "HitResult Structure (by ref)"))
  (bind _button (`self.Button`))
  (bind _button_2 (`self.Button`))
  (bind _returnvalue_location (`KismetMathLibrary.BreakTransform` (`SceneComponent.GetRelativeTransform` _button)))
  (bind (_returnvalue_location_2 _returnvalue_rotation) (`KismetMathLibrary.BreakTransform` (`SceneComponent.GetRelativeTransform` _button_2)))
  (if (`self.isPressable`)
    (set `self.isPressable` false)
    (cast `/Game/VRTemplate/Blueprints/VRPawn` OtherActor)
    (`KismetSystemLibrary.MoveComponentTo` _button_2 (- _returnvalue_location_2 (0.0 0.0 193.0)) _returnvalue_rotation false false 0.25)
    (`/Game/Blueprints/Rover/BP_Rover.OnButtonPressed_Event` (`self.Rover`) (`self.Color`))
    (set `self.isPressed` true)
    (`KismetSystemLibrary.MoveComponentTo` _button (+ _returnvalue_location (0.0 0.0 193.0)) (struct) false false 0.5)
    (set `self.isPressable` true)
    (set `self.isPressed` false)))

(fn `UserConstructionScript`)