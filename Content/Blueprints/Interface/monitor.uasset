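; Monitor actor that shows an on or off look by swapping the material on its Plane component.
; Each Tick it compares the On flag of a referenced Puller with the cached PrevOn value.
; When the flag changes, it applies Mat2 for on or Mat1 for off and updates the cache, so the material is set only on transitions.
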(event `self.ReceiveTick`
  (params (DeltaSeconds :type "Float (single-precision)"))
  (bind _on (`/Game/Blueprints/Interface/Puller.On` (`self.puller`)))
  (if (!= (`self.prevOn`) _on)
    (if _on
      (`PrimitiveComponent.SetMaterial` (`self.Plane`) 0 (`self.mat2`))
      (else
        (`PrimitiveComponent.SetMaterial` (`self.Plane`) 0 (`self.mat1`))))
    (set `self.prevOn` _on)))

(fn `UserConstructionScript`)