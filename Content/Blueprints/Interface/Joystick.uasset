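; VR joystick actor that the player grabs with a motion controller, with a trigger-operated button.
; While held, Tick turns the stick toward the controller with clamped look-at rotation and derives XRot and YRot from the tip's offset to the pivot.
; The holding hand's trigger animates a button press and calls the Explorer's extra-function event, re-arming on trigger release.
; Release resets the stick's rotation, axis values and hand.
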(event `self.ReceiveBeginPlay`
  (set `self.hand` 0)
  (set `self.canGrab` true)
  (bind _returnvalue (`GameplayStatics.GetActorOfClass` "/Game/VRTemplate/Blueprints/VRPawn.VRPawn_C"))
  (set `self.vrPawn` _returnvalue))

(event `OnTriggerPressedRight_Event`
  (bind _cube1 (`self.Cube1`))
  (bind (_returnvalue_location _returnvalue_rotation) (`KismetMathLibrary.BreakTransform` (`SceneComponent.GetRelativeTransform` _cube1)))
  (if (== (`self.hand`) 1)
    (`|ExecutionSequence` :!label _label
      (:`then_1`
        (if (`self.canGrab`)
          (set `self.canGrab` false)
          (`KismetSystemLibrary.MoveComponentTo` _cube1 (- _returnvalue_location (0.0 0.0 5.0)) _returnvalue_rotation false false 0.1)
          (`KismetSystemLibrary.MoveComponentTo` _cube1 (+ _returnvalue_location (0.0 0.0 5.0)) _returnvalue_rotation false false 0.1)
          (`/Game/Blueprints/Rover/BP_Rover.extraFunction_Event` (`self.Explorer`)))))))

(event `OnTriggerReleasedRight_Event`
  (set `self.canGrab` true :!label _label_2))

(event `/Game/Interfaces/Grab.Release`
  (params (MotionController :type "MotionControllerComponent Object Reference"))
  (if (not (== null (`self.Motion Controller`)))
    (set `self.Motion Controller` null)
    (`SceneComponent.K2_SetWorldRotation` (`self.Cube`) (struct :`Pitch` 90.0 :`Yaw` -90.0) false false)
    (set `self.XRot` 0.0)
    (set `self.YRot` 0.0)
    (set `self.hand` 0)))

(event `OnTriggerReleasedLeft_Event`
  (goto _label_2))

(event `OnTriggerPressedLeft_Event`
  (if (== (`self.hand`) 2)
    (goto _label)))

(event `/Game/Interfaces/Grab.Grab`
  (params (MotionController :type "MotionControllerComponent Object Reference"))
  (set `self.Motion Controller` MotionController)
  (if (== MotionController (`/Game/VRTemplate/Blueprints/VRPawn.MotionControllerRight` (`self.vrPawn`)))
    (set `self.hand` 1)
    (else
      (set `self.hand` 2))))

(event `self.ReceiveTick`
  (params (DeltaSeconds :type "Float (single-precision)"))
  (bind _cube (`self.Cube`))
  (`|ExecutionSequence`
    (:`then_0`
      (bind _motion_controller (`self.Motion Controller`)
        (:`then`
          (`SceneComponent.K2_SetWorldRotation` _cube (`KismetMathLibrary.MakeRotator` (`KismetMathLibrary.FClamp` (.roll (`KismetMathLibrary.FindLookAtRotation` (`SceneComponent.K2_GetComponentLocation` _cube) (`SceneComponent.K2_GetComponentLocation` _motion_controller))) 0.0 180.0) (`KismetMathLibrary.FClamp` (.pitch (`KismetMathLibrary.FindLookAtRotation` (`SceneComponent.K2_GetComponentLocation` _cube) (`SceneComponent.K2_GetComponentLocation` _motion_controller))) 0.0 100.0) (.yaw (`KismetMathLibrary.FindLookAtRotation` (`SceneComponent.K2_GetComponentLocation` _cube) (`SceneComponent.K2_GetComponentLocation` _motion_controller)))) false false))
        (:`else`)))
    (:`then_1`
      (set `self.XRot` (/ (.x (- (`SceneComponent.K2_GetComponentLocation` (`self.Cube2`)) (`SceneComponent.K2_GetComponentLocation` (`self.Cube`)))) 20.0))
      (set `self.YRot` (/ (.y (- (`SceneComponent.K2_GetComponentLocation` (`self.Cube2`)) (`SceneComponent.K2_GetComponentLocation` (`self.Cube`)))) 20.0)))))

(fn `UserConstructionScript`)