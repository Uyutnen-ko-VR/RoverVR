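; VR joystick that a motion controller grabs to rotate the Explorer component of a referenced object V.
; While held, the Cube pivot aims at the controller within clamped angles, and it snaps back to a rest rotation on release.
; Each Tick, the world X/Y offset between Cube2 and Cube adds yaw and clamped pitch to Explorer, without delta-time scaling.
; Steering requires Con to be on and V to have battery.
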(event `self.ReceiveBeginPlay`
  (set `self.Explorer` (`/Game/Blueprints/Rover/BP_Rover.Scene` (`self.v`))))

(event `/Game/Interfaces/Grab.Release`
  (params (MotionController :type "MotionControllerComponent Object Reference"))
  (if (not (== null (`self.Motion Controller`)))
    (set `self.Motion Controller` null)
    (`SceneComponent.K2_SetWorldRotation` (`self.Cube`) (struct :`Pitch` 90.0 :`Roll` 90.0) false false)))

(event `/Game/Interfaces/Grab.Grab`
  (params (MotionController :type "MotionControllerComponent Object Reference"))
  (set `self.Motion Controller` MotionController))

(event `self.ReceiveTick`
  (params (DeltaSeconds :type "Float (single-precision)"))
  (bind _cube (`self.Cube`))
  (bind _explorer (`self.Explorer`))
  (bind _returnvalue (`SceneComponent.GetRelativeTransform` _explorer))
  (if (== (`self.Explorer`) null)
    (set `self.Explorer` (`/Game/Blueprints/Rover/BP_Rover.s` (`self.v`))))
  (`|ExecutionSequence`
    (:`then_0`
      (bind _motion_controller (`self.Motion Controller`)
        (:`then`
          (`SceneComponent.K2_SetWorldRotation` _cube (`KismetMathLibrary.MakeRotator` (`KismetMathLibrary.FClamp` (.roll (`KismetMathLibrary.FindLookAtRotation` (`SceneComponent.K2_GetComponentLocation` _cube) (`SceneComponent.K2_GetComponentLocation` _motion_controller))) 0.0 180.0) (`KismetMathLibrary.FClamp` (.pitch (`KismetMathLibrary.FindLookAtRotation` (`SceneComponent.K2_GetComponentLocation` _cube) (`SceneComponent.K2_GetComponentLocation` _motion_controller))) 0.0 150.0) (.yaw (`KismetMathLibrary.FindLookAtRotation` (`SceneComponent.K2_GetComponentLocation` _cube) (`SceneComponent.K2_GetComponentLocation` _motion_controller)))) false false))
        (:`else`)))
    (:`then_1`
      (if (and (`/Game/Blueprints/Interface/Puller.On` (`self.con`)) (> (`/Game/Blueprints/Rover/BP_Rover.battery` (`self.v`)) 0.0))
        (`SceneComponent.K2_SetRelativeRotation` _explorer (`KismetMathLibrary.MakeRotator` (.roll (.rotation _returnvalue)) (`KismetMathLibrary.FClamp` (+ (.pitch (.rotation _returnvalue)) (/ (.y (- (`SceneComponent.K2_GetComponentLocation` (`self.Cube2`)) (`SceneComponent.K2_GetComponentLocation` (`self.Cube`)))) -20.0)) -50.0 50.0) (+ (/ (.x (- (`SceneComponent.K2_GetComponentLocation` (`self.Cube2`)) (`SceneComponent.K2_GetComponentLocation` (`self.Cube`)))) -20.0) (.yaw (.rotation _returnvalue)))) false false)))))

(fn `UserConstructionScript`)