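; BP_mooner is a six-wheeled vehicle, apparently a moon rover, driven by XRot and YRot values while Battery is above zero.
; Each tick YRot spins the cylinder wheels and XRot yaws the steering cubes within angle limits.
; Cube's physics velocity is set along the averaged right vectors of Cube1 and StaticMesh, scaled by YRot.
; Wheel breakage is unfinished: a timer check picks a random index, but BreakWheel is empty and uncalled.
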(event `self.ReceiveBeginPlay`
  (set `self.battery` 600.0)
  (set `self.nBroken` 0)
  (set `self.NewVar_0` (`self.Cube4`)))

(event `self.ReceiveTick`
  (params (DeltaSeconds :type "Float (single-precision)"))
  (bind _timer (`self.timer`))
  (bind _xrot (`self.XRot`))
  (bind _returnvalue (- (.yaw (`SceneComponent.K2_GetComponentRotation` (`self.Cube2`))) 0.0))
  (if (> (`self.battery`) 0.0)
    (if true
      (`|ExecutionSequence`
        (:`then_0`
          (`SceneComponent.K2_AddLocalRotation` (`self.Cylinder`) (`KismetMathLibrary.MakeRotator` 0.0 0.0 (* (`self.kMove`) (`self.YRot`))) false false)
          (`SceneComponent.K2_AddLocalRotation` (`self.Cylinder5`) (`KismetMathLibrary.MakeRotator` 0.0 0.0 (* (`self.kMove`) (`self.YRot`))) false false)
          (`SceneComponent.K2_AddLocalRotation` (`self.Cylinder4`) (`KismetMathLibrary.MakeRotator` 0.0 0.0 (* (`self.kMove`) (`self.YRot`))) false false)
          (`SceneComponent.K2_AddLocalRotation` (`self.Cylinder2`) (`KismetMathLibrary.MakeRotator` 0.0 0.0 (* (`self.kMove`) (`self.YRot`))) false false)
          (`SceneComponent.K2_AddLocalRotation` (`self.Cylinder3`) (`KismetMathLibrary.MakeRotator` 0.0 0.0 (* (`self.kMove`) (`self.YRot`))) false false)
          (`SceneComponent.K2_AddLocalRotation` (`self.Cylinder1`) (`KismetMathLibrary.MakeRotator` 0.0 0.0 (* (`self.kMove`) (`self.YRot`))) false false)
          (if (> _xrot 0.0)
            (if (< _returnvalue 140.0)
              (`SceneComponent.K2_AddLocalRotation` (`self.Cube1`) (`KismetMathLibrary.MakeRotator` 0.0 0.0 (* (`self.kRot`) _xrot)) false false :!label _label)
              (`SceneComponent.K2_AddLocalRotation` (`self.Cube2`) (`KismetMathLibrary.MakeRotator` 0.0 0.0 (* (`self.kRot`) _xrot)) false false))
            (elif (> _returnvalue 40.0)
              (goto _label)
              (else
                _)))
          (if (< _timer 0.0)
            (set `self.nBroken` (`KismetMathLibrary.RandomIntegerInRange` 0 5))
            (set `self.timer` (+ _timer (`KismetMathLibrary.RandomFloatInRange` 30.0 50.0)))))
        (:`then_1`
          (`PrimitiveComponent.SetPhysicsLinearVelocity` (`self.Cube`) (* (/ (+ (`SceneComponent.GetRightVector` (`self.Cube1`)) (`SceneComponent.GetRightVector` (`self.StaticMesh`))) (2.0 2.0 2.0)) (* (`self.VelocityMultiplayer`) (`self.YRot`))) false "None"))
        (:`then_2`
          ;[1 1 1] Speed km/h
          (bind _returnvalue_2 (`PrimitiveComponent.GetPhysicsLinearVelocity` (`self.Cube`) "None"))
          (if (!= _returnvalue_2 (0.0 0.0 0.0))
            _))))))

(fn `BreakWheel`)

(fn `Start`)

(fn `UserConstructionScript`)