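; Sys tracks the current mission stage and objective text (Russian strings) for a vehicle control, calibration and travel sequence.
; It starts at stage 3 with a task to enable control, then Tick polls flags to set later objectives: drive to the station once GetOn is on, and reach the beacons when T is set.
; Overlapping Caliberzone disables its collision and starts the calibration objective.
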(event `self.ReceiveBeginPlay`
  (set `self.stage` 3)
  (set `self.task` "Включить управление"))

(event `self.ReceiveTick`
  (params (DeltaSeconds :type "Float (single-precision)"))
  (`|ExecutionSequence`
    (:`then_0`
      (if (`self.k`)
        _
        (elif (`/Game/Blueprints/Interface/Puller.On` (`self.getOn`))
          (set `self.stage` 0)
          (set `self.task` "Доехать до станции")
          (set `self.k` true))))
    (:`then_1`
      (if (`self.t`)
        (if true
          (set `self.t` false)
          (set `self.task` "Добраться до маячков")
          (set `self.stage` 0)
          (`SceneComponent.SetHiddenInGame` (`self.caliberzone`) true true))))))

(event `self.caliberzone.OnComponentBeginOverlap`
  (params (OverlappedComponent :type "PrimitiveComponent Object Reference") (OtherActor :type "Actor Object Reference") (OtherComp :type "PrimitiveComponent Object Reference") (OtherBodyIndex :type Integer) (bFromSweep :type Boolean) (SweepResult :type "HitResult Structure (by ref)"))
  (`PrimitiveComponent.SetCollisionEnabled` (`self.caliberzone`) "NoCollision")
  (set `self.task` "Провести калибровку")
  (set `self.stage` 1))

(fn `Try`
  (if true
    _))

(fn `UserConstructionScript`)