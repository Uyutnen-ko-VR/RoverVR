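; Puller is a two-state lever operated by a grabbing motion controller, storing its state in an On flag.
; While held, Tick pitches RubilaCube toward the controller, using a look-at angle in the cube's offset-rotated local space, clamped to a quarter turn.
; Release clears the controller and snaps the cube to either end of its travel, setting On when pulled past halfway.
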(event `self.ReceiveBeginPlay`
  (set `self.On` false)
  (`SceneComponent.K2_SetRelativeRotation` :`self` (`self.Rubila_Cube`)))

(event `/Game/Interfaces/Grab.Release`
  (params (MotionController :type "MotionControllerComponent Object Reference"))
  (bind _rubila_cube (`self.Rubila_Cube`))
  (if (not (== null (`self.Motion Controller`)))
    (set `self.Motion Controller` null)
    (if (> (.pitch (.rotation (`SceneComponent.GetRelativeTransform` _rubila_cube))) 45.0)
      (set `self.On` true)
      (`SceneComponent.K2_SetRelativeRotation` _rubila_cube (struct :`Pitch` 90.0) false false)
      (else
        (set `self.On` false)
        (`SceneComponent.K2_SetRelativeRotation` :`self` _rubila_cube)))))

(event `/Game/Interfaces/Grab.Grab`
  (params (MotionController :type "MotionControllerComponent Object Reference"))
  (set `self.Motion Controller` MotionController))

(event `self.ReceiveTick`
  (params (DeltaSeconds :type "Float (single-precision)"))
  (bind _rubila_cube (`self.Rubila_Cube`))
  (bind (_returnvalue_location _returnvalue_rotation _returnvalue_scale) (`KismetMathLibrary.BreakTransform` (`SceneComponent.K2_GetComponentToWorld` (`self.Rubila_Cube`))))
  (bind _motion_controller (`self.Motion Controller`)
    (:`then`
      (bind _returnvalue_location_2 (`KismetMathLibrary.BreakTransform` (`KismetMathLibrary.MakeRelativeTransform` (`SceneComponent.K2_GetComponentToWorld` _motion_controller) (`KismetMathLibrary.MakeTransform` _returnvalue_location (`KismetMathLibrary.ComposeRotators` _returnvalue_rotation (struct :`Pitch` 40.0)) _returnvalue_scale))))
      (bind (_returnvalue_roll _returnvalue_pitch) (`KismetMathLibrary.BreakRotator` (`KismetMathLibrary.FindLookAtRotation` (`KismetMathLibrary.MakeVector` 0.0) _returnvalue_location_2)))
      (`SceneComponent.K2_SetRelativeRotation` _rubila_cube (`KismetMathLibrary.MakeRotator` 0.0 (`KismetMathLibrary.FClamp` (+ (.pitch (.rotation (`SceneComponent.GetRelativeTransform` _rubila_cube))) _returnvalue_pitch) 0.0 90.0)) false false))
    (:`else`)))

(fn `UserConstructionScript`)