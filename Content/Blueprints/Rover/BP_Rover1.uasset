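; Rover vehicle driven by a stick and color buttons, active while Con is on.
; Switch I selects driving, with stick to steering and brake (throttle is unwired), or rotating Cube yaw and Cube2 pitch within clamps.
; Outside driving, with Cube2 raised enough, color events slide one of three boxes out, swapping or retracting the current one.
; A selected box raises Cube2's minimum pitch; ID 3 means none.
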(event `self.ReceiveBeginPlay`
  (bind _boxes (`self.boxes`))
  (set `self.s` (`self.Scene`))
  (`KismetArrayLibrary.Array_Add` _boxes (`self.GreenBox`))
  (`KismetArrayLibrary.Array_Add` _boxes (`self.BlueBox`))
  (`KismetArrayLibrary.Array_Add` _boxes (`self.RedBox`))
  (set `self.SelectedBoxID` 3))

(event `self.ReceiveTick`
  (params (DeltaSeconds :type "Float (single-precision)"))
  (bind _vehiclemovementcomponent (`self.VehicleMovementComponent`))
  (bind _stick (`self.Stick`))
  (bind _cube2 (`self.cube2`))
  (bind _cube (`self.Cube`))
  (bind _returnvalue (`SceneComponent.GetRelativeTransform` _cube2))
  (bind _returnvalue_2 (`SceneComponent.GetRelativeTransform` _cube))
  (bind _yrot (`/Game/Blueprints/Interface/Joystick.YRot` _stick))
  (bind _returnvalue_3 (- 0.0 (`/Game/Blueprints/Interface/Joystick.XRot` _stick)))
  (bind _returnvalue_4 (+ (* _yrot -1.0) (.pitch (.rotation _returnvalue))))
  (if (`/Game/Blueprints/Interface/Puller.On` (`self.con`))
    (if (`/Game/Blueprints/Interface/Puller.On` (`self.i`))
      (`ChaosVehicleMovementComponent.SetBrakeInput` _vehiclemovementcomponent _yrot)
      (`ChaosVehicleMovementComponent.SetSteeringInput` _vehiclemovementcomponent _returnvalue_3)
      (else
        (`SceneComponent.K2_SetRelativeRotation` _cube (`KismetMathLibrary.MakeRotator` (.roll (.rotation _returnvalue_2)) (.pitch (.rotation _returnvalue_2)) (`KismetMathLibrary.FClamp` (+ (.yaw (.rotation _returnvalue_2)) _returnvalue_3) 50.0 130.0)) false false)
        (if (< (`self.SelectedBoxID`) 3)
          (`SceneComponent.K2_SetRelativeRotation` _cube2 (`KismetMathLibrary.MakeRotator` (.roll (.rotation _returnvalue)) (`KismetMathLibrary.FClamp` _returnvalue_4 20.0 40.0) (.yaw (.rotation _returnvalue))) false false)
          (else
            (`SceneComponent.K2_SetRelativeRotation` _cube2 (`KismetMathLibrary.MakeRotator` (.roll (.rotation _returnvalue)) (`KismetMathLibrary.FClamp` _returnvalue_4 0.0 40.0) (.yaw (.rotation _returnvalue))) false false)))))))

(event `OnButtonPressed_Event`
  (params (Color :type Integer))
  (bind _boxes (`self.boxes`))
  (bind _selectedboxid (`self.SelectedBoxID`))
  (bind _output (`|GetArrayItem` _boxes Color))
  (bind _output_2 (`|GetArrayItem` _boxes _selectedboxid))
  (bind (_returnvalue_location _returnvalue_rotation) (`KismetMathLibrary.BreakTransform` (`SceneComponent.GetRelativeTransform` _output_2)))
  (bind (_returnvalue_location_2 _returnvalue_rotation_2) (`KismetMathLibrary.BreakTransform` (`SceneComponent.GetRelativeTransform` _output)))
  (bind (_returnvalue_location_3 _returnvalue_rotation_3) (`KismetMathLibrary.BreakTransform` (`SceneComponent.GetRelativeTransform` _output)))
  (bind (_returnvalue_location_4 _returnvalue_rotation_4) (`KismetMathLibrary.BreakTransform` (`SceneComponent.GetRelativeTransform` _output_2)))
  (if (and (>= (.pitch (.rotation (`SceneComponent.GetRelativeTransform` (`self.cube2`)))) 20.0) (`/Game/Blueprints/Interface/Puller.On` (`self.con`)))
    (if (`/Game/Blueprints/Interface/Puller.On` (`self.i`))
      _
      (elif (== _selectedboxid 3)
        (`KismetSystemLibrary.MoveComponentTo` _output (+ _returnvalue_location_2 (-200.0 0.0 0.0)) _returnvalue_rotation_2)
        (set `self.SelectedBoxID` Color)
        (elif (== Color _selectedboxid)
          (`KismetSystemLibrary.MoveComponentTo` _output_2 (+ _returnvalue_location (200.0 0.0 0.0)) _returnvalue_rotation)
          (set `self.SelectedBoxID` 3)
          (else
            (`KismetSystemLibrary.MoveComponentTo` _output_2 (+ _returnvalue_location_4 (200.0 0.0 0.0)) _returnvalue_rotation_4)
            (`KismetSystemLibrary.MoveComponentTo` _output (+ _returnvalue_location_3 (-200.0 0.0 0.0)) _returnvalue_rotation_3)
            (set `self.SelectedBoxID` Color)))))))

(fn `GetBoxByID`
  (params (BoxID :type Integer))
  (returns (Box :type "StaticMeshComponent Object Reference"))
  (if (== BoxID 0)
    (return (`self.RedBox`))
    (elif (== 1 BoxID)
      (return (`self.GreenBox`))
      (elif (== BoxID 2)
        (return (`self.BlueBox`))))))

(fn `OnColorButtonPressed`
  (params (Color :type Integer))
  (`self.OnButtonPressed` Color))

(fn `UserConstructionScript`)