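; BP_Rover is a drivable rover that takes its throttle and steering from a stick object's rotation.
; On each tick, while the Con reference reports On, the stick's Y rotation sets throttle and its negated X rotation sets steering on the vehicle movement component.
; BeginPlay stores the Cube in variable S, which the shown graphs do not use further, and the construction script is empty.
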(event `self.ReceiveBeginPlay`
  (set `self.s` (`self.Cube`)))

(event `self.ReceiveTick`
  (params (DeltaSeconds :type "Float (single-precision)"))
  (bind _vehiclemovementcomponent (`self.VehicleMovementComponent`))
  (bind _stick (`self.Stick`))
  (if (`/Game/Blueprints/Puller.On` (`self.con`))
    (`ChaosVehicleMovementComponent.SetThrottleInput` _vehiclemovementcomponent (`/Game/Blueprints/Lever.YRot` _stick))
    (`ChaosVehicleMovementComponent.SetSteeringInput` _vehiclemovementcomponent (- 0.0 (`/Game/Blueprints/Lever.XRot` _stick)))))

(fn `UserConstructionScript`)